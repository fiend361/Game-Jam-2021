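; GeneratorBP is a spawner that keeps creating GoodCube actors at random spots around its owner's location.
; Tick feeds a Delay set by CubeSpawnDelay, so the latent node paces spawning instead of firing every frame.
; Each cube gets a random horizontal offset within a square area at the owner's height, plus a random rotation on all three axes.
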(event EventBeginPlay)

(event EventTick
  (params (DeltaSeconds :type Float%20%28single-precision%29))
  (bind _returnvalue (Math|Random|RandomFloat))
  (bind _returnvalue_2 (* _returnvalue 3.6e+02))
  (Utilities|FlowControl|Delay (Variables|Default|GetCubeSpawnDelay))
  (Game|SpawnActorfromClass "/Game/GoodCube.GoodCube_C" (Math|Transform|MakeTransform (+ (Transformation|GetActorLocation (Components|GetOwner)) (Math|Vector|MakeVector (Math|Random|RandomFloatinRange -5e+02 5e+02) (Math|Random|RandomFloatinRange -5e+02 5e+02) 0.0)) (Math|Rotator|MakeRotator _returnvalue_2 _returnvalue_2 _returnvalue_2)) "Undefined" 0 0))